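; BP_CoinDropComponent rewards the player with coins when the actor that owns it dies.
; On BeginPlay it binds to the health-depleted event of the owner's BP_HealthComponent.
; On death it adds a random amount between Min and Max directly to player 0's BP_Player inventory, without spawning a pickup.
; The debug message rolls its own random number, so it can differ from the amount added.
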(event `self.ReceiveBeginPlay`
  (add `/Game/Blueprints/HealthAndDamage/BP_HealthComponent.OnHealthDepleted` (`Actor.GetComponentByClass` (`self.GetOwner`) "/Game/Blueprints/HealthAndDamage/BP_HealthComponent.BP_HealthComponent_C") (delegate `ActorDied`)))

(event `ActorDied`
  (bind _returnvalue (`KismetMathLibrary.RandomIntegerInRange` (`self.min`) (`self.max`)))
  (bind _asbp_player (cast `/Game/Blueprints/BP_Player` (`GameplayStatics.GetPlayerCharacter` 0)))
  (`/Game/Blueprints/BP_Player.addToInventory` _asbp_player "NewEnumerator5" (`KismetMathLibrary.Conv_IntToDouble` _returnvalue))
  (`KismetSystemLibrary.PrintString` (`KismetStringLibrary.Concat_StrStr` "Added " (`KismetStringLibrary.Conv_IntToString` _returnvalue) " coins to player") true true (struct :`R` 1.0 :`G` 0.935911 :`A` 1.0)))