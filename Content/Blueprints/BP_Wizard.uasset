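; BP_Wizard is a Paper2D enemy that pursues and burns the player.
; PawnSensing or overlap starts pursuit, flipping yaw by X position.
; Overlap triggers a wind-up, then AttackBox damages one other PaperCharacter per one-second tick while overlap and burn sound last.
; BP_HealthComponent events darken the sprite, play hit reactions outside attacks and handle death, with per-tick polling loops awaiting flipbook completion.
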(event `self.ReceiveBeginPlay`)

(event `self.ReceiveTick`
  (params (DeltaSeconds :type "Float (single-precision)"))
  (if (not (`self.isDead`))
    (`self.ResetFlipbook`)
    (if (`self.isWalking`)
      (`self.RotateActorTowardsPlayer`)
      (if (not (`self.isAttacking`))
        (`self.AddMovementInput` (`self.GetActorForwardVector`) 0.1)))))

(event `self.BP_HealthComponent.OnHealthChange`
  (params (NewHealth :type "Float (double-precision)"))
  ;[1 1 1] Taking Damage
  (`self.SetDamagedColor` NewHealth (`/Game/Blueprints/HealthAndDamage/BP_HealthComponent.MaxHealth` (`self.BP_HealthComponent`)))
  (if (> NewHealth 0.0)
    (if (not (`self.isAttacking`))
      (set `self.isTakingDamage` true)
      (`PaperFlipbookComponent.SetLooping` (`self.Sprite`) false)
      (`PaperFlipbookComponent.SetFlipbook` (`self.Sprite`) "/Game/Assets/Flipbooks/FB_Wizard_Take_Hit.FB_Wizard_Take_Hit")
      (`PaperFlipbookComponent.PlayFromStart` (`self.Sprite`))
      (if (`PaperFlipbookComponent.IsPlaying` (`self.Sprite`)) :!label _label
        (`KismetSystemLibrary.DelayUntilNextTick`)
        (goto _label)
        (else
          (set `self.isTakingDamage` false))))))

(event `self.BP_HealthComponent.OnHealthDepleted`
  ;[1 1 1] Death
  (set `self.isDead` true)
  (`self.SetActorEnableCollision` false)
  (`GameplayStatics.PlaySound2D` "/Game/Sounds/Magic_Hit.Magic_Hit" 1.0 1.0 0.0 null null)
  (`PaperFlipbookComponent.SetFlipbook` (`self.Sprite`) "/Game/Assets/Flipbooks/FB_Wizard_Death.FB_Wizard_Death")
  (`PaperFlipbookComponent.SetLooping` (`self.Sprite`) false)
  (if (`PaperFlipbookComponent.IsPlaying` (`self.Sprite`)) :!label _label_2
    (`KismetSystemLibrary.DelayUntilNextTick`)
    (goto _label_2)
    (else
      (`KismetSystemLibrary.Delay` 4.0)
      (`self.K2_DestroyActor`))))

(event `Attack`
  ;[1 1 1] Start Attack
  (if (not (or (`self.isTakingDamage`) (`self.isAttacking`) (`self.isDead`)))
    (set `self.isAttacking` true)
    (`PaperFlipbookComponent.SetLooping` (`self.Sprite`) true)
    (`PaperFlipbookComponent.SetFlipbook` (`self.Sprite`) "/Game/Assets/Flipbooks/FB_Wizard_Move.FB_Wizard_Move")
    (`GameplayStatics.PlaySound2D` "/Game/Sounds/Ignite.Ignite" 1.0 1.0 0.0 null null)
    (`PaperFlipbookComponent.PlayFromStart` (`self.Sprite`))
    (`KismetSystemLibrary.Delay` (`PaperFlipbookComponent.GetFlipbookLength` (`self.Sprite`)))
    (if (not (or (`self.isDead`) (`self.isTakingDamage`)))
      (`PaperFlipbookComponent.SetFlipbook` (`self.Sprite`) "/Game/Assets/Flipbooks/FB_Wizard_Attack.FB_Wizard_Attack")
      (bind _returnvalue (`GameplayStatics.SpawnSound2D` "/Game/Sounds/Burn2.Burn2" 1.0 1.0 0.0 null))
      (set `self.sound` _returnvalue)
      (bind _playerhit (`self.HandleHits` :!label _label_3))
      (if _playerhit
        (`GameplayStatics.PlaySound2D` "/Game/Sounds/Sizzle.Sizzle" 1.0 1.0 0.0 null null))
      (if (and (`self.actorOverlapping`) (`AudioComponent.IsPlaying` (`self.sound`)))
        (`KismetSystemLibrary.Delay` 1.0)
        (goto _label_3)
        (else
          _)))
    (set `self.isAttacking` false)
    (`AudioComponent.Stop` (`self.sound`))))

(event `self.ReceiveActorBeginOverlap`
  (params (OtherActor :type "Actor Object Reference"))
  ;[1 1 1] Trigger Attack
  (if (`KismetMathLibrary.ClassIsChildOf` (`GameplayStatics.GetObjectClass` OtherActor) "/Game/Blueprints/BP_Player.BP_Player_C")
    (set `self.spottedPlayer` OtherActor)
    (`self.NoticePlayer`)
    (set `self.actorOverlapping` true)
    (if (`self.actorOverlapping`) :!label _label_4
      (if (not (`self.isAttacking`))
        (`self.Attack`))
      (`KismetSystemLibrary.DelayUntilNextTick`)
      (goto _label_4))))

(event `self.ReceiveActorEndOverlap`
  (params (OtherActor :type "Actor Object Reference"))
  ;[1 1 1] Trigger Attack
  (set `self.actorOverlapping` false))

(event `NoticePlayer`
  (set `self.isWalking` true)
  (`self.RotateActorTowardsPlayer`))

(event `self.PawnSensing.OnSeePawn`
  (params (Pawn :type "Pawn Object Reference"))
  (set `self.spottedPlayer` Pawn)
  (`self.NoticePlayer`)
  (`KismetSystemLibrary.RetriggerableDelay` 1.0)
  (set `self.isWalking` false))

(fn `HandleHits`
  (returns (PlayerHit :type Boolean))
  (for _array_element (`PrimitiveComponent.GetOverlappingActors` (`self.AttackBox`) "/Script/Paper2D.PaperCharacter")
    (`KismetSystemLibrary.PrintString` (`KismetSystemLibrary.GetDisplayName` _array_element))
    (if (!= self _array_element)
      (`GameplayStatics.ApplyDamage` _array_element (`self.baseDamage`))
      (return true)))
  (return false))

(fn `ResetFlipbook`
  (if (or (`self.isDead`) (`self.isAttacking`) (`self.isTakingDamage`))
    (return)
    (else
      (`PaperFlipbookComponent.SetLooping` (`self.Sprite`) true)
      (`PaperFlipbookComponent.Play` (`self.Sprite`))
      (`PaperFlipbookComponent.SetFlipbook` (`self.Sprite`) "/Game/Assets/Flipbooks/FB_Wizard_Idle.FB_Wizard_Idle"))))

(fn `RotateActorTowardsPlayer`
  (if (> (.x (`self.K2_GetActorLocation`)) (.x (`self.K2_GetActorLocation` (`self.spottedPlayer`))))
    (set `self.yaw` 180.0)
    (else
      (set `self.yaw` 0.0)))
  (`self.K2_SetActorRotation` (`KismetMathLibrary.MakeRotator` 0.0 0.0 (`self.yaw`))))

(fn `SetDamagedColor`
  (params (health :type "Float (double-precision)") (maxHealth :type "Float (double-precision)"))
  (bind _returnvalue (+ (* (/ health maxHealth) 0.5) 0.5))
  (`PaperFlipbookComponent.SetSpriteColor` (`self.Sprite`) (`KismetMathLibrary.MakeColor` _returnvalue _returnvalue _returnvalue)))

(fn `UserConstructionScript`)