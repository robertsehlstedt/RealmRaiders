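; BP_Chest is a paid loot chest that grants the player a random stat buff or coins.
; Overlap shows the interact prompt and cost, or the drop once opened, on the player's HUD and clears it on exit.
; InteractwithChest charges coins, plays the sound, sets the sprite play rate and marks it opened.
; GenerateRandomDrop picks a random item type and ranged value, which goes into the player's inventory and HUD text.
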(event `self.ReceiveBeginPlay`
  (`PaperFlipbookComponent.SetLooping` (`self.ChestSprite`) false))

(event `self.ReceiveActorBeginOverlap`
  (params (OtherActor :type "Actor Object Reference"))
  (bind _asbp_player (cast `/Game/Blueprints/BP_Player` OtherActor))
  (if (`self.isOpened`)
    (`self.setHUDWhenOpened` _asbp_player)
    (else
      (`self.setHUDWhenClosed` _asbp_player))))

(event `self.ReceiveActorEndOverlap`
  (params (OtherActor :type "Actor Object Reference"))
  (bind _asbp_player (cast `/Game/Blueprints/BP_Player` OtherActor))
  (`self.resetHUD` _asbp_player))

(event `/Game/Blueprints/I_Interact.InteractWithChest`
  (if (not (`self.isOpened`))
    (bind _asbp_player (cast `/Game/Blueprints/BP_Player` (`GameplayStatics.GetPlayerCharacter` 0)))
    (bind _succeeded (`/Game/Blueprints/BP_Player.Pay Coins` _asbp_player (`self.openingCost`)))
    (if _succeeded
      (`GameplayStatics.PlaySound2D` "/Game/Sounds/Open_Chest.Open_Chest" 1.0 1.0 0.0 null null)
      (`KismetSystemLibrary.Delay` 0.4)
      (`PaperFlipbookComponent.SetPlayRate` (`self.ChestSprite`) 1.0)
      (set `self.isOpened` true)
      (bind (_item _value) (`self.GenerateRandomDrop`))
      (bind _asbp_player_2 (cast `/Game/Blueprints/BP_Player` (`GameplayStatics.GetPlayerCharacter` 0)))
      (set `self.itemDropped` _item)
      (set `self.valueDropped` _value)
      (`/Game/Blueprints/BP_Player.AddToInventory` _asbp_player_2 _item _value)
      (`self.setHUDWhenOpened` _asbp_player_2))))

(fn `GenerateRandomDrop`
  (returns (Item :type "/Game/Blueprints/Items/ItemType Enum") (Value :type "Float (double-precision)"))
  (locals (ItemTypes :type "Array of /Game/Blueprints/Items/ItemType Enum") (Value :type "Float (double-precision)"))
  (bind _enumvalue (foreach `/Game/Blueprints/Items/ItemType` false)
    (:`LoopBody`
      (`KismetArrayLibrary.Array_Add` (`local.ItemTypes`) _enumvalue))
    (:`then`
      (switch `/Game/Blueprints/Items/ItemType` (`|GetArrayItem` (`local.ItemTypes`) (`KismetMathLibrary.RandomInteger` (`KismetArrayLibrary.Array_Length` (`local.ItemTypes`))))
        (:`NewEnumerator0`
          (return "NewEnumerator0" (`KismetMathLibrary.RandomFloatInRange` 0.02 0.05)))
        (:`NewEnumerator2`
          (return "NewEnumerator2" (`KismetMathLibrary.RandomFloatInRange` 5.0 10.0)))
        (:`NewEnumerator3`
          (return "NewEnumerator3" (`KismetMathLibrary.RandomFloatInRange` 5.0 10.0)))
        (:`NewEnumerator5`
          (return "NewEnumerator5" (`KismetMathLibrary.RandomFloatInRange` 5.0 20.0)))))))

(fn `getValueString`
  (params (type :type "/Game/Blueprints/Items/ItemType Enum" :default "NewEnumerator1") (value :type "Float (double-precision)"))
  (returns (valueString :type String))
  (switch `/Game/Blueprints/Items/ItemType` type
    (:`NewEnumerator0`
      (return (`KismetStringLibrary.Concat_StrStr` "Dropped bonus movement speed (" (`KismetStringLibrary.Conv_IntToString` (`KismetMathLibrary.FTrunc` (* (`local.value`) 100.0))) "%)")))
    (:`NewEnumerator2`
      (return (`KismetStringLibrary.Concat_StrStr` "Dropped bonus attack damage (" (`KismetStringLibrary.Conv_IntToString` (`KismetMathLibrary.FTrunc` (`local.value`))) ")")))
    (:`NewEnumerator3`
      (return (`KismetStringLibrary.Concat_StrStr` "Dropped bonus max health (" (`KismetStringLibrary.Conv_IntToString` (`KismetMathLibrary.FTrunc` (`local.value`))) ")")))
    (:`NewEnumerator5`
      (return (`KismetStringLibrary.Concat_StrStr` "Dropped " (`KismetStringLibrary.Conv_IntToString` (`KismetMathLibrary.FTrunc` (`local.value`))) " coins")))))

(fn `resetHUD`
  (params (BP_Player :type "/Game/Blueprints/BP_Player Object Reference"))
  (bind _hudreference (`/Game/Blueprints/BP_Player.hudReference` BP_Player))
  (set `TextBlock.Text` "" (`/Game/UI/WB_HUD.upperText` _hudreference))
  (set `TextBlock.Text` "" (`/Game/UI/WB_HUD.lowerText` _hudreference)))

(fn `setHUDWhenClosed`
  (params (BP_Player :type "/Game/Blueprints/BP_Player Object Reference"))
  (bind _hudreference (`/Game/Blueprints/BP_Player.hudReference` BP_Player))
  (set `TextBlock.Text` "Interact [E]" (`/Game/UI/WB_HUD.upperText` _hudreference))
  (set `TextBlock.Text` (`KismetTextLibrary.Conv_StringToText` (`KismetStringLibrary.Concat_StrStr` (`KismetStringLibrary.Conv_IntToString` (`self.openingCost`)) " coins")) (`/Game/UI/WB_HUD.lowerText` _hudreference)))

(fn `setHUDWhenOpened`
  (params (BP_Player :type "/Game/Blueprints/BP_Player Object Reference"))
  (bind _hudreference (`/Game/Blueprints/BP_Player.hudReference` (`local.BP_Player`)))
  (bind _valuestring (`self.getValueString` (`self.itemDropped`) (`self.valueDropped`)))
  (set `TextBlock.Text` (`KismetTextLibrary.Conv_StringToText` _valuestring) (`/Game/UI/WB_HUD.upperText` _hudreference))
  (set `TextBlock.Text` "" (`/Game/UI/WB_HUD.lowerText` _hudreference)))

(fn `UserConstructionScript`)