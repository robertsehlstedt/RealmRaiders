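; BP_Skeleton_Spawner periodically spawns BP_Skeleton actors at its own transform while the player is nearby.
; BeginPlay caches BP_Player and waits a random delay before starting SpawnTick, a self-repeating loop paced by SpawnDelay.
; Each tick spawns only if the world-wide skeleton count is below MaxSpawnedEnemies and the player is within a horizontal distance band and a vertical limit.
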(event `self.ReceiveBeginPlay`
  (bind _returnvalue (`GameplayStatics.GetActorOfClass` "/Game/Blueprints/BP_Player.BP_Player_C"))
  (set `self.Player` _returnvalue)
  (`KismetSystemLibrary.Delay` (`KismetMathLibrary.Conv_IntToDouble` (`KismetMathLibrary.RandomInteger` (`self.spawnDelay`))))
  (`self.SpawnTick`))

(event `SpawnTick`
  (bind _player (`self.Player`))
  (bind _returnvalue (`self.GetHorizontalDistanceTo` _player self))
  (bind _outactors (`GameplayStatics.GetAllActorsOfClass` "/Game/Blueprints/BP_Skeleton.BP_Skeleton_C"))
  (if (< (`KismetArrayLibrary.Array_Length` _outactors) (`self.maxSpawnedEnemies`))
    (if (and (>= _returnvalue 150.0) (<= _returnvalue 550.0) (<= (`self.GetVerticalDistanceTo` _player self) 220.0))
      (`|SpawnActorFromClass` "/Game/Blueprints/BP_Skeleton.BP_Skeleton_C" (`self.GetTransform` self) "Undefined" "MultiplyWithRoot" null null)))
  (`KismetSystemLibrary.Delay` (`KismetMathLibrary.Conv_IntToDouble` (`self.spawnDelay`)))
  (`self.SpawnTick`))

(fn `UserConstructionScript`)