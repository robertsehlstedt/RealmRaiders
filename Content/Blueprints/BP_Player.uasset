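; 2D Paper2D player character handling Enhanced Input movement, jumping, slash attacks, direction locking and chest interaction through an interface.
; IsRunning, IsJumping and IsAttacking flags arbitrate flipbooks, with Tick restoring idle and locked direction enabling backwards running.
; Attacks damage the first other character overlapping the flipped AttackBox, retrying once after a miss.
; Health changes trigger camera shake and red flash, while HandleInventoryUpdated copies buff and coin values into variables.
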(event `self.ReceiveBeginPlay`
  ;[1 1 1] Set mapping context
  (bind _asbp_playercontroller (cast `/Game/Blueprints/BP_Playercontroller` (`self.GetController`)))
  (`EnhancedInputSubsystemInterface.AddMappingContext` (pcsubsystem `EnhancedInputLocalPlayerSubsystem` _asbp_playercontroller) "/Game/Blueprints/IMC_Default.IMC_Default" 0 (struct)))

(event `self.ReceiveTick`
  (params (DeltaSeconds :type "Float (single-precision)"))
  ;[1 1 1] Reset Flipbook to idle when necessary
  (`self.resetFlipbook`))

(event `EnhancedInput|/Game/Blueprints/IA_Movement`
  (params (ActionValue :type "Float (double-precision)") (ElapsedSeconds :type "Float (double-precision)") (TriggeredSeconds :type "Float (double-precision)") (InputAction :type "InputAction Object Reference" :default "/Game/Blueprints/IA_Movement.IA_Movement"))
  ;[1 1 1] Horizontal movement
  (:`Triggered`
    (`|ExecutionSequence`
      (:`then_0`
        (set `self.isRunning` true)
        (`self.AddMovementInput` (`self.GetActorForwardVector`) ActionValue))
      (:`then_1`
        (if (`self.isJumping`)
          _
          (elif (not (`self.isAttacking`))
            (bind _runningbackwards (`self.isRunningBackwards` ActionValue))
            (if _runningbackwards
              (`PaperFlipbookComponent.SetFlipbook` (`self.Sprite`) "/Game/Assets/Flipbooks/FB_Reverse.FB_Reverse")
              (else
                (`PaperFlipbookComponent.SetFlipbook` (`self.Sprite`) "/Game/Assets/Flipbooks/FB_Run.FB_Run"))))))
      (:`then_2`
        (if (`self.rotationLocked`)
          _
          (elif (> ActionValue 0.0)
            (`SceneComponent.K2_SetWorldRotation` :`self` (`self.Sprite`))
            (`SceneComponent.K2_SetRelativeLocation` (`self.AttackBox`) (15.0 0.0 0.0) false false)
            (else
              (`SceneComponent.K2_SetWorldRotation` (`self.Sprite`) (struct :`Yaw` 180.0) false false)
              (`SceneComponent.K2_SetRelativeLocation` (`self.AttackBox`) (-15.0 0.0 0.0) false false)))))))
  (:`Completed`
    (set `self.isRunning` false)))

(event `EnhancedInput|/Game/Blueprints/IA_Jump`
  (params (ActionValue :type Boolean) (ElapsedSeconds :type "Float (double-precision)") (TriggeredSeconds :type "Float (double-precision)") (InputAction :type "InputAction Object Reference" :default "/Game/Blueprints/IA_Jump.IA_Jump"))
  ;[1 1 1] Vertical movement
  (:`Triggered`
    (if (not (`self.isJumping`))
      (set `self.isJumping` true)
      (`self.Jump`)
      (`PaperFlipbookComponent.SetLooping` (`self.Sprite`) false)
      (`PaperFlipbookComponent.SetFlipbook` (`self.Sprite`) "/Game/Assets/Flipbooks/FB_Jump.FB_Jump"))))

(event `self.OnLanded`
  (params (Hit :type "HitResult Structure (by ref)"))
  ;[1 1 1] Vertical movement
  (set `self.isJumping` false))

(event `EnhancedInput|/Game/Blueprints/IA_MainAttack`
  (params (ActionValue :type Boolean) (ElapsedSeconds :type "Float (double-precision)") (TriggeredSeconds :type "Float (double-precision)") (InputAction :type "InputAction Object Reference" :default "/Game/Blueprints/IA_MainAttack.IA_MainAttack"))
  ;[1 1 1] MainAttack
  (:`Triggered`
    (if (not (or (`self.isAttacking`) (`self.isJumping`)))
      (set `self.isAttacking` true)
      (`PaperFlipbookComponent.SetLooping` (`self.Sprite`) false)
      (`PaperFlipbookComponent.SetFlipbook` (`self.Sprite`) "/Game/Assets/Flipbooks/FB_Slash.FB_Slash")
      (`GameplayStatics.PlaySound2D` "/Game/Sounds/Swoosh.Swoosh" 1.0 1.0 0.0 null null)
      (`KismetSystemLibrary.Delay` 0.07)
      (bind _enemyhit (`self.HandleHits`))
      (if (not _enemyhit)
        (`KismetSystemLibrary.Delay` 0.05)
        (`self.HandleHits`))
      (if (`PaperFlipbookComponent.IsPlaying` (`self.Sprite`)) :!label _label
        (`KismetSystemLibrary.DelayUntilNextTick`)
        (goto _label)
        (else
          (set `self.isAttacking` false))))))

(event `EnhancedInput|/Game/Blueprints/IA_LockDirection`
  (params (ActionValue :type Boolean) (ElapsedSeconds :type "Float (double-precision)") (TriggeredSeconds :type "Float (double-precision)") (InputAction :type "InputAction Object Reference" :default "/Game/Blueprints/IA_LockDirection.IA_LockDirection"))
  ;[1 1 1] LockRotation
  (:`Triggered`
    (set `self.rotationLocked` true))
  (:`Canceled`
    (set `self.rotationLocked` false :!label _label_2))
  (:`Completed`
    (goto _label_2)))

(event `EnhancedInput|/Game/Blueprints/IA_Interact`
  (params (ActionValue :type Boolean) (ElapsedSeconds :type "Float (double-precision)") (TriggeredSeconds :type "Float (double-precision)") (InputAction :type "InputAction Object Reference" :default "/Game/Blueprints/IA_Interact.IA_Interact"))
  ;[1 1 1] Open Chest
  (:`Triggered`
    (`KismetSystemLibrary.PrintText` "Hello")
    (for _array_element (`self.GetOverlappingActors` "/Game/Blueprints/BP_Chest.BP_Chest_C")
      (if (`KismetSystemLibrary.DoesImplementInterface` _array_element "/Game/Blueprints/I_Interact.I_Interact_C")
        (message `/Game/Blueprints/I_Interact.InteractWithChest` _array_element)
        (break)))))

(event `self.BP_HealthComponent.OnHealthChange`
  (params (NewHealth :type "Float (double-precision)"))
  ;[1 1 1] Taking Damage
  (`GameplayStatics.PlayWorldCameraShake` "/Game/Blueprints/BP_TakeDmgCameraShake.BP_TakeDmgCameraShake_C" (`self.K2_GetActorLocation`) 0.0 500.0)
  (`PaperFlipbookComponent.SetSpriteColor` (`self.Sprite`) (`KismetMathLibrary.MakeColor` 1.0))
  (`KismetSystemLibrary.Delay` 0.1)
  (`PaperFlipbookComponent.SetSpriteColor` (`self.Sprite`) (`KismetMathLibrary.MakeColor` 1.0 1.0 1.0)))

(fn `HandleHits`
  (returns (EnemyHit :type Boolean))
  (for _array_element (`PrimitiveComponent.GetOverlappingActors` (`self.AttackBox`) "/Script/Paper2D.PaperCharacter")
    (`KismetSystemLibrary.PrintString` (`KismetSystemLibrary.GetDisplayName` _array_element))
    (if (!= self _array_element)
      (`GameplayStatics.PlayWorldCameraShake` "/Game/Blueprints/BP_DealDmgCameraShake.BP_DealDmgCameraShake_C" (`self.K2_GetActorLocation`) 0.0 500.0)
      (`GameplayStatics.ApplyDamage` _array_element (`KismetMathLibrary.Conv_IntToDouble` (`self.baseDamage`)))
      (`GameplayStatics.PlaySound2D` "/Game/Sounds/Metal_Hit.Metal_Hit" 1.0 1.0 0.0 null null)
      (return true)))
  (return false))

(fn `HandleInventoryUpdated`
  (params (ItemType :type "/Game/Blueprints/Items/ItemType Enum" :default "NewEnumerator0"))
  (switch `/Game/Blueprints/Items/ItemType` ItemType
    (:`NewEnumerator1`
      (`KismetSystemLibrary.PrintString` "Warning: Picked up NoneType item"))
    (:`NewEnumerator0`
      (set `self.BonusMovementSpeed` (`KismetMathLibrary.FTrunc` (`BlueprintMapLibrary.Map_Find` (`self.Inventory`) "NewEnumerator0"))))
    (:`NewEnumerator2`
      (set `self.BonusDamage` (`KismetMathLibrary.FTrunc` (`BlueprintMapLibrary.Map_Find` (`self.Inventory`) "NewEnumerator2"))))
    (:`NewEnumerator3`
      (set `self.BonusMaxHealth` (`KismetMathLibrary.FTrunc` (`BlueprintMapLibrary.Map_Find` (`self.Inventory`) "NewEnumerator3"))))
    (:`NewEnumerator5`
      (set `self.Coin` (`KismetMathLibrary.FTrunc` (`BlueprintMapLibrary.Map_Find` (`self.Inventory`) "NewEnumerator5"))))))

(fn `isRunningBackwards`
  (params (actionValue :type "Float (double-precision)"))
  (returns (runningBackwards :type Boolean))
  (return (xor (>= (`KismetMathLibrary.SignOfFloat` (.x (`KismetMathLibrary.Conv_RotatorToVector` (`SceneComponent.K2_GetComponentRotation` (`self.Sprite`))))) 0.0) (>= (`KismetMathLibrary.SignOfFloat` actionValue) 0.0))))

(fn `resetFlipbook`
  (if (`self.isJumping`)
    _
    (elif (not (`self.isAttacking`))
      (`PaperFlipbookComponent.SetLooping` (`self.Sprite`) true)
      (`PaperFlipbookComponent.Play` (`self.Sprite`))
      (if (not (`self.isRunning`))
        (`PaperFlipbookComponent.SetFlipbook` (`self.Sprite`) "/Game/Assets/Flipbooks/FB_Idle.FB_Idle")))))

(fn `UserConstructionScript`)