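; BP_QuestTrigger is a one-shot trigger actor that gives the player a new quest objective when they overlap it.
; On the first overlap by a BP_Player, it passes NewQuestObjective to the player's SetCurrentMission and prints the objective on screen.
; It then sets HasTriggered to block repeat firing and plays a 2D sound cue.
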(event `self.ReceiveActorBeginOverlap`
  (params (OtherActor :type "Actor Object Reference"))
  (if (not (`self.hasTriggered`))
    (bind _asbp_player (cast `/Game/Blueprints/BP_Player` OtherActor))
    (`/Game/Blueprints/BP_Player.setCurrentMission` _asbp_player (`KismetTextLibrary.Conv_TextToString` (`self.newQuestObjective`)))
    (`KismetSystemLibrary.PrintString` (`KismetStringLibrary.Concat_StrStr` "New objective: " (`KismetTextLibrary.Conv_TextToString` (`self.newQuestObjective`))) true true (struct :`R` 0.141954 :`B` 0.234375 :`A` 1.0))
    (set `self.hasTriggered` true)
    (`GameplayStatics.PlaySound2D` "/Engine/EditorSounds/GamePreview/PossessPlayer_Cue.PossessPlayer_Cue" 1.0 1.0 0.0 null null)))

(fn `UserConstructionScript`)