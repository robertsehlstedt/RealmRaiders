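; BP_Skeleton is a 2D flipbook skeleton that reacts visually to incoming damage.
; On AnyDamage it prints the damage amount, raises IsTakingDamage and switches its sprite to the hit flipbook.
; A Delay equal to that flipbook's length then restores the idle flipbook and clears the flag.
; It tracks no health or death, and nothing here reads the flag.
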(event `self.ReceiveAnyDamage`
  (params (Damage :type "Float (single-precision)") (DamageType :type "DamageType Object Reference") (InstigatedBy :type "Controller Object Reference") (DamageCauser :type "Actor Object Reference"))
  (`KismetSystemLibrary.PrintString` (`KismetStringLibrary.Conv_DoubleToString` Damage))
  (set `self.isTakingDamage` true)
  (`PaperFlipbookComponent.SetFlipbook` (`self.Sprite`) "/Game/Assets/Flipbooks/FB_Skeleton_Hit.FB_Skeleton_Hit")
  (`KismetSystemLibrary.Delay` (`PaperFlipbookComponent.GetFlipbookLength` (`self.Sprite`)))
  (`PaperFlipbookComponent.SetFlipbook` (`self.Sprite`) "/Game/Assets/Flipbooks/FB_Skeleton_Idle.FB_Skeleton_Idle")
  (set `self.isTakingDamage` false))

(fn `UserConstructionScript`)