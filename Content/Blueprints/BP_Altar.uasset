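; BP_Altar is a coin-operated altar, built on a chest sprite, that brings up the win screen once paid for.
; Player overlap shows either the interact prompt with cost or, if already opened, dropped-item text on the player's HUD, cleared on exit.
; InteractwithChest charges coins through the player, plays a win sound, sets the sprite's play rate, then after a delay marks it opened, pauses the game and adds the Winscreen widget.
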(event `self.ReceiveBeginPlay`
  (`PaperFlipbookComponent.SetLooping` (`self.ChestSprite`) false))

(event `self.ReceiveActorBeginOverlap`
  (params (OtherActor :type "Actor Object Reference"))
  (bind _asbp_player (cast `/Game/Blueprints/BP_Player` OtherActor))
  (if (`self.isOpened`)
    (`self.setHUDWhenOpened` _asbp_player)
    (else
      (`self.setHUDWhenClosed` _asbp_player))))

(event `self.ReceiveActorEndOverlap`
  (params (OtherActor :type "Actor Object Reference"))
  (bind _asbp_player (cast `/Game/Blueprints/BP_Player` OtherActor))
  (`self.resetHUD` _asbp_player))

(event `/Game/Blueprints/I_Interact.InteractWithChest`
  (if (not (`self.isOpened`))
    (bind _asbp_player (cast `/Game/Blueprints/BP_Player` (`GameplayStatics.GetPlayerCharacter` 0)))
    (bind _succeeded (`/Game/Blueprints/BP_Player.Pay Coins` _asbp_player (`self.openingCost`)))
    (if _succeeded
      (`GameplayStatics.PlaySound2D` "/Game/Sounds/Win_Sound.Win_Sound" 1.0 1.0 0.0 null null)
      (`PaperFlipbookComponent.SetPlayRate` (`self.ChestSprite`) 1.0)
      (`KismetSystemLibrary.Delay` 2.0)
      (set `self.isOpened` true)
      (`GameplayStatics.SetGamePaused` true)
      (bind _returnvalue (`|CreateWidget` "/Game/Blueprints/UI/Winscreen.Winscreen_C"))
      (`UserWidget.AddToViewport` _returnvalue 0))))

(fn `resetHUD`
  (params (BP_Player :type "/Game/Blueprints/BP_Player Object Reference"))
  (bind _hudreference (`/Game/Blueprints/BP_Player.hudReference` BP_Player))
  (set `TextBlock.Text` "" (`/Game/UI/WB_HUD.upperText` _hudreference))
  (set `TextBlock.Text` "" (`/Game/UI/WB_HUD.lowerText` _hudreference)))

(fn `setHUDWhenClosed`
  (params (BP_Player :type "/Game/Blueprints/BP_Player Object Reference"))
  (bind _hudreference (`/Game/Blueprints/BP_Player.hudReference` BP_Player))
  (set `TextBlock.Text` "Interact [E]" (`/Game/UI/WB_HUD.upperText` _hudreference))
  (set `TextBlock.Text` (`KismetTextLibrary.Conv_StringToText` (`KismetStringLibrary.Concat_StrStr` (`KismetStringLibrary.Conv_IntToString` (`self.openingCost`)) " coins")) (`/Game/UI/WB_HUD.lowerText` _hudreference)))

(fn `setHUDWhenOpened`
  (params (BP_Player :type "/Game/Blueprints/BP_Player Object Reference"))
  (bind _hudreference (`/Game/Blueprints/BP_Player.hudReference` BP_Player))
  (set `TextBlock.Text` (`KismetTextLibrary.Conv_StringToText` (`KismetStringLibrary.Concat_StrStr` "Dropped " (`|GetEnumeratorNameAsString` (`self.itemDropped`)) " (" (`KismetStringLibrary.Conv_IntToString` (`KismetMathLibrary.FTrunc` (`self.valueDropped`))) ")")) (`/Game/UI/WB_HUD.upperText` _hudreference))
  (set `TextBlock.Text` "" (`/Game/UI/WB_HUD.lowerText` _hudreference)))

(fn `UserConstructionScript`)